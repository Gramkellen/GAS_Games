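; GA_FileBolt is a gameplay ability that casts a fire bolt projectile toward the point under the mouse.
; On activation, a TargetDataUnderMouse task supplies the hit location, and the avatar turns to face it through CombatInterface.
; It then plays the AM_Cast_FireBolt montage, waits for the Event.Montage.FireBolt gameplay event, and spawns the projectile at that timing toward the saved location.
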(event `self.K2_ActivateAbility`
  ;[1 1 1] 这里如果节点结束再调用Data会被清除的
  (bind (_asynctaskproxy _datahandle) (`TargetDataUnderMouse.CreateTargetDataUnderMouse`)
    (:`ValidDataSignature`
      (set `self.ProjectileLocation` (`.Location` (`GameplayStatics.BreakHitResult` (`AbilitySystemBlueprintLibrary.GetHitResultFromTargetData` _datahandle))))
      (bind _ascombat_interface (cast `CombatInterface` (`self.GetAvatarActorFromActorInfo`)))
      (`CombatInterface.FacingTarget` _ascombat_interface (`self.ProjectileLocation`))
      (`AbilityTask_PlayMontageAndWait.CreatePlayMontageAndWaitProxy` "None" "/Game/Assets/Characters/Aura/Animations/Abilities/AM_Cast_FireBolt.AM_Cast_FireBolt"
        (:`then`
          (`AbilityTask_WaitGameplayEvent.WaitGameplayEvent` (struct :`TagName` "Event.Montage.FireBolt") null
            (:`EventReceived`
              (`self.SpawnProjectile` (`self.ProjectileLocation`)))))))))